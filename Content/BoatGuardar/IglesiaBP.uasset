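; IglesiaBP is a church actor that toggles its static mesh's visibility in response to the third-person character.
; Entering its Box shows the mesh, while leaving hides it and clears the Escuchar flag.
; PawnSensing also shows the mesh when it hears that character while Escuchar is false.
; Disconnected logic, which never runs, would display a temporary BienvenidoPrueba welcome widget and set Escuchar.
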(event `self.Box.OnComponentBeginOverlap`
  (params (OverlappedComponent :type "PrimitiveComponent Object Reference") (OtherActor :type "Actor Object Reference") (OtherComp :type "PrimitiveComponent Object Reference") (OtherBodyIndex :type Integer) (bFromSweep :type Boolean) (SweepResult :type "HitResult Structure (by ref)"))
  (cast `/Game/ThirdPerson/Blueprints/BP_ThirdPersonCharacter` OtherActor)
  (`SceneComponent.SetVisibility` (`self.StaticMesh`) true false))

(event `self.Box.OnComponentEndOverlap`
  (params (OverlappedComponent :type "PrimitiveComponent Object Reference") (OtherActor :type "Actor Object Reference") (OtherComp :type "PrimitiveComponent Object Reference") (OtherBodyIndex :type Integer))
  (cast `/Game/ThirdPerson/Blueprints/BP_ThirdPersonCharacter` OtherActor)
  (`SceneComponent.SetVisibility` (`self.StaticMesh`) false false)
  (set `self.Escuchar` false))

(event `self.PawnSensing.OnHearNoise`
  (params (Instigator :type "Pawn Object Reference") (Location :type "Vector Structure (by ref)") (Volume :type "Float (single-precision)"))
  (if (not (`self.Escuchar`))
    (cast `/Game/ThirdPerson/Blueprints/BP_ThirdPersonCharacter` Instigator)
    (`SceneComponent.SetVisibility` (`self.StaticMesh`) true false)))

(fn `UserConstructionScript`)