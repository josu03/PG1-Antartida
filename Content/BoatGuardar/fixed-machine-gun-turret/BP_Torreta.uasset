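; BP_Torreta is a turret actor that turns toward the player character and fires projectiles when it sees it.
; PawnSensing sightings of BP_ThirdPersonCharacter snap the whole actor to face the target, then a short delay precedes spawning a Proyectil at each of two arrow components.
; A debug print compares the first spawned projectile to the character, and an unconnected line trace with a hit-name print remains unused.
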(event `self.PawnSensing.OnSeePawn`
  (params (Pawn :type "Pawn Object Reference"))
  (bind _asbp_third_person_character (cast `/Game/ThirdPerson/Blueprints/BP_ThirdPersonCharacter` Pawn))
  (`self.K2_SetActorRotation` (`KismetMathLibrary.FindLookAtRotation` (`self.K2_GetActorLocation`) (`self.K2_GetActorLocation` Pawn)))
  (`KismetSystemLibrary.Delay` 0.2)
  (`|ExecutionSequence`
    (:`then_0`
      (bind _returnvalue (`|SpawnActorFromClass` "/Game/ThirdPerson/Blueprints/ArmasSystem/Balas/Proyectil.Proyectil_C" (`SceneComponent.K2_GetComponentToWorld` (`self.Arrow`)) "Undefined" "MultiplyWithRoot" null null))
      (if (== _returnvalue _asbp_third_person_character)
        (`KismetSystemLibrary.PrintString` "Hello")))
    (:`then_1`
      (`|SpawnActorFromClass` "/Game/ThirdPerson/Blueprints/ArmasSystem/Balas/Proyectil.Proyectil_C" (`SceneComponent.K2_GetComponentToWorld` (`self.Arrow1`)) "Undefined" "MultiplyWithRoot" null null))))

(fn `UserConstructionScript`)