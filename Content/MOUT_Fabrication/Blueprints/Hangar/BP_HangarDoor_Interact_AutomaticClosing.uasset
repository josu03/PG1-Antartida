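; Interactive hangar door actor that slides four door panels open on the E key and closes them automatically.
; Per-panel timelines lerp relative location to open offsets and reverse to close, with a Closed flag and delays gating the cycle around OpenDuration.
; The closing sequence calls OpenRightDoor2 instead of CloseRightDoor2, so that panel never reverses.
; Trigger overlap casts have no target class, leaving the EnableInput and DisableInput calls disconnected.
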(event `Open Left Door`
  (bind (_direction _alpha) (`Timeline|TL_LeftDoor` :!label _label)
    (:`Update`
      (`SceneComponent.K2_SetRelativeLocation` (`self.LeftDoor1`) (`KismetMathLibrary.VLerp` (0.0 8.0 0.0) (`self.LeftDoorOpen`) _alpha) false false))))

(event `Open Left Door 2`
  (bind (_direction _alpha) (`Timeline|TL_LeftDoor2` :!label _label_2)
    (:`Update`
      (`SceneComponent.K2_SetRelativeLocation` (`self.LeftDoor2`) (`KismetMathLibrary.VLerp` (0.0 8.0 0.0) (`self.LeftDoorOpen2`) _alpha) false false))))

(event `Close Left Door`
  (goto _label :!via `Reverse`))

(event `Close Left Door 2`
  (goto _label_2 :!via `Reverse`))

(event `Open Right Door 2`
  (bind (_direction _alpha) (`Timeline|TL_RightDoor2` :!label _label_3)
    (:`Update`
      (`SceneComponent.K2_SetRelativeLocation` (`self.RightDoor2`) (`KismetMathLibrary.VLerp` (0.0 8.0 0.0) (`self.RightDoorOpen2`) _alpha) false false))))

(event `Open Right Door`
  (bind (_direction _alpha) (`Timeline|TL_RightDoor` :!label _label_4)
    (:`Update`
      (`SceneComponent.K2_SetRelativeLocation` (`self.RIghtDoor1`) (`KismetMathLibrary.VLerp` (0.0 8.0 0.0) (`self.RightDoorOpen`) _alpha) false false))))

(event `Close Right Door 2`
  (goto _label_3 :!via `Reverse`))

(event `Close Right Door`
  (goto _label_4 :!via `Reverse`))

(event `Key|E`
  (params (Key :type "Key Structure"))
  (:`Pressed`
    (if (`self.Closed`)
      (`self.Open Left Door`)
      (`self.Open Right Door`)
      (`self.Open Left Door 2`)
      (`self.Open Right Door 2`)
      (set `self.Closed` false)
      (`KismetSystemLibrary.Delay` 5.0)
      (`KismetSystemLibrary.Delay` (`self.Open Duration`))
      (`self.Close Left Door`)
      (`self.Close Right Door`)
      (`self.Close Left Door 2`)
      (`self.Open Right Door 2`)
      (`KismetSystemLibrary.Delay` 5.0)
      (set `self.Closed` true))))

(event `self.Trigger.OnComponentBeginOverlap`
  (params (OverlappedComponent :type "PrimitiveComponent Object Reference") (OtherActor :type "Actor Object Reference") (OtherComp :type "PrimitiveComponent Object Reference") (OtherBodyIndex :type Integer) (bFromSweep :type Boolean) (SweepResult :type "HitResult Structure (by ref)"))
  (cast `` OtherActor))

(event `self.Trigger.OnComponentEndOverlap`
  (params (OverlappedComponent :type "PrimitiveComponent Object Reference") (OtherActor :type "Actor Object Reference") (OtherComp :type "PrimitiveComponent Object Reference") (OtherBodyIndex :type Integer))
  (cast `` OtherActor))

(fn `UserConstructionScript`)