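; Alex is an NPC character that patrols, talks to the player on sight and can die from damage.
; A looping AI move cycles between two target points with random pauses.
; PawnSensing sends it to the player, then it shows the next dialogue line in a widget and resumes patrol after a delay.
; Depleted health triggers ragdoll and stops movement; the notice montage is left unwired.
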(event `self.ReceiveAnyDamage`
  (params (Damage :type "Float (single-precision)") (DamageType :type "DamageType Object Reference") (InstigatedBy :type "Controller Object Reference") (DamageCauser :type "Actor Object Reference"))
  (bind _health (`self.health`))
  (set `self.health` (- _health Damage))
  (if (<= _health 0.0)
    (`KismetSystemLibrary.PrintString` "death")
    (`PrimitiveComponent.SetSimulatePhysics` (`self.Mesh`) true)
    (`CharacterMovementComponent.SetMovementMode` (`self.CharacterMovement`) "MOVE_None" 0)))

(event `self.ReceiveBeginPlay`
  (`self.PatrullarPuntos`))

(event `PatrullarPuntos`
  (bind _index (`self.Index`))
  (`|AIMoveTo` self (`self.K2_GetActorLocation` (`|GetArrayItem` (`self.Target`) (`self.Index`))) null
    (:`OnSuccess`
      (`KismetSystemLibrary.Delay` (`KismetMathLibrary.RandomFloatInRange` 1.0 1.5))
      (`self.PatrullarPuntos`)
      (`/Engine/EditorBlueprintResources/StandardMacros.IncrementInt` _index
        (:`  `
          (if (== _index 2)
            (set `self.Index` 0)))))))

(event `self.PawnSensing.OnSeePawn`
  (params (Pawn :type "Pawn Object Reference"))
  (bind _asbp_third_person_character (cast `/Game/ThirdPerson/Blueprints/BP_ThirdPersonCharacter` Pawn))
  (`|AIMoveTo` self (`self.K2_GetActorLocation` _asbp_third_person_character) (`GameplayStatics.GetPlayerController` 0) 110.0
    (:`OnSuccess`
      (`/Engine/EditorBlueprintResources/StandardMacros.IncrementInt` (`self.Talkindex`)
        (:`  `
          (if (<= (`self.Talkindex`) (`KismetArrayLibrary.Array_Length` (`self.dialoge`)))
            (`self.UI`
              (:`then`
                _)
              (:`else`
                (bind _returnvalue (`|CreateWidget` "/Game/Characters/Alex/WidegetTextoGuarda.WidegetTextoGuarda_C" (`GameplayStatics.GetPlayerController` 0)))
                (bind _output_get (set `self.UI` _returnvalue))
                (`UserWidget.AddToViewport` _output_get 0)))
            (`TextBlock.SetText` (`/Game/Characters/Alex/WidegetTextoGuarda.TalkText` (`self.UI`)) (`|GetArrayItem` (`self.dialoge`) (`self.Talkindex`)))
            (`KismetSystemLibrary.Delay` 5.0)
            (`self.PatrullarPuntos`)
            (else
              (`Widget.RemoveFromParent` (`self.UI`)))))))))

(fn `UserConstructionScript`)